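; BP_Yatai is a festival food/game stall actor that configures its look and layout in the construction script.
; It applies the Yatai material to mesh slot 2 behind an "MI_Y_" name-prefix check on StaticMesh, then scales the plane.
; It places PlaneEnd from the plane's Y scale and shifts the mesh back by half the start-to-end span.
; Event graph logic, rotation presets and random material selection are unconnected.
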(event `self.ReceiveBeginPlay`)

(fn `UserConstructionScript`
  (bind _planeend (`self.PlaneEnd`))
  (if (`KismetStringLibrary.EqualEqual_StrStr` (`KismetStringLibrary.Left` (`KismetSystemLibrary.GetObjectName` (`self.StaticMesh`)) 5) "MI_Y_")
    (`PrimitiveComponent.SetMaterial` (`self.StaticMesh`) 2 (`self.Yatai`)))
  (`SceneComponent.SetRelativeScale3D` (`self.Plane`) (`self.PlaneScale`))
  (`SceneComponent.K2_SetRelativeLocation` _planeend (`KismetMathLibrary.MakeVector` (.x (`SceneComponent.RelativeLocation` (`self.PlaneStart`))) (* (`self.PlaneOffsetPerScale`) (.y (`self.PlaneScale`))) (.z (`SceneComponent.RelativeLocation` (`self.PlaneStart`)))) false false)
  (bind _output_get (set `self.PlaneOffset` (/ (- (.y (`SceneComponent.RelativeLocation` _planeend)) (.y (`SceneComponent.RelativeLocation` (`self.PlaneStart`)))) 2.0)))
  (`SceneComponent.K2_SetRelativeLocation` (`self.StaticMesh`) (`KismetMathLibrary.MakeVector` 0.0 (* _output_get -1.0)) false false))