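; BP_Goal is the level goal object, which ends the stage when it receives damage.
; ReceiveDamage runs the parent logic, then creates a WBP_Goal widget, plays its goal animation and starts DelayFadeOut.
; DelayFadeOut waits briefly, plays the fade-out on the BP_MainGameMode fade widget, then waits again before opening ResultMap.
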(event `DelayFadeOut`
  (`KismetSystemLibrary.Delay` 1.0)
  (`/Game/Cat/UI/WBP_FadeOutIn.PlayFadeOut` (`/Game/Cat/BP/BP_MainGameMode.FadeInOutWidget` (cast `/Game/Cat/BP/BP_MainGameMode` (`GameplayStatics.GetGameMode`) :!pure true)))
  (`KismetSystemLibrary.Delay` 2.0)
  (`GameplayStatics.OpenLevel` "ResultMap"))

(event `self.ReceiveBeginPlay`)

(fn `ReceiveDamage`
  (returns (point :type Integer))
  (bind _point (`parent.ReceiveDamage`))
  (bind _returnvalue (`|CreateWidget` "/Game/Cat/UI/WBP_Goal.WBP_Goal_C"))
  (`UserWidget.AddToViewport` _returnvalue 0)
  (`/Game/Cat/UI/WBP_Goal.PlayGoalAnimation` _returnvalue)
  (`self.DelayFadeOut`)
  (return _point))

(fn `UserConstructionScript`)