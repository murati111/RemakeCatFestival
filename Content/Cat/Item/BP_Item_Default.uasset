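; BP_Item_Default is an item Blueprint that takes a random look from three materials: RingoAme, Takoyaki or YoYo.
; The construction script rolls a random index to set PlaneMaterial, then calls the parent construction script.
; ReceiveDamage only returns the parent's damage result, and the event graph holds just disabled stubs, so any other behavior comes from the parent class.
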(fn `ReceiveDamage`
  (returns (point :type Integer))
  (bind _point (`parent.ReceiveDamage`))
  (return _point))

(fn `UserConstructionScript`
  (set `self.PlaneMaterial` (select `int` (`KismetMathLibrary.RandomInteger` 3) :`0` "/Game/Cat/Item/MI_Item_RingoAme.MI_Item_RingoAme" :`1` "/Game/Cat/Item/MI_Item_Takoyaki.MI_Item_Takoyaki" :`2` "/Game/Cat/Item/MI_Item_YoYo.MI_Item_YoYo" :!type "MaterialInterface Object Reference"))
  (`parent.UserConstructionScript`))