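; Title-screen game mode that drives the menu flow from fade-in to loading the main map.
; On BeginPlay it fades in and binds title, ghost-select and fade widget events, arming the pawn's one-time press-start after the title fade event.
; Single play fades out directly, while ghost mode first loads the chosen rank's data through the game instance, and fade-out completion opens the map.
; A separate event passes ghost times to the selection widget.
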(event `self.ReceiveBeginPlay`
  (`parent.ReceiveBeginPlay`)
  (`|ExecutionSequence`
    (:`then_0`
      (bind _wbp_fadeoutin (`self.GetWBP_FadeInOut`))
      (`/Game/Cat/UI/WBP_FadeOutIn.PlayFadeInForTitle` _wbp_fadeoutin))
    (:`then_1`
      (bind _aswbp_title (`self.GetWBP_Title`))
      (add `/Game/Cat/UI/Title/WBP_Title.OnFadeTitle` _aswbp_title (delegate `FadeTitle`))
      (add `/Game/Cat/UI/Title/WBP_Title.OnSinglePlayClicked` _aswbp_title (delegate `FadeOutMap`)))
    (:`then_2`
      (bind _wbp_ghostselect (`self.GetWBP_GhostSelect`))
      (add `/Game/Cat/UI/Title/WBP_GhostSelect.OnPressGhostMode` _wbp_ghostselect (delegate `PressGhostMode`))
      (bind _wbp_fadeoutin_2 (`self.GetWBP_FadeInOut`))
      (add `/Game/Cat/UI/WBP_FadeOutIn.OnFadeOut` _wbp_fadeoutin_2 (delegate `OpenMainMap`)))))

(event `FadeTitle`
  ;[1 1 1] FadeIn後AnyKeyEventが発行できるように
  (bind _asbp_title_pawn (`self.GetTitlePlayer`))
  (add `/Game/Cat/BP/Title/BP_TitlePawn.OnPressStart` _asbp_title_pawn (delegate `PressStart`)))

(event `FadeOutMap`
  ;[1 1 1] SinglePlayの場合そのままFadeOut
  (bind _wbp_fadeoutin (`self.GetWBP_FadeInOut`))
  (`/Game/Cat/UI/WBP_FadeOutIn.PlayFadeOut` _wbp_fadeoutin))

(event `PressStart`
  ;[1 1 1] AnyKeyが押されたらタイトルを表示
  (`/Engine/EditorBlueprintResources/StandardMacros.DoOnce` false
    (:`Completed`
      (bind _aswbp_title (`self.GetWBP_Title`))
      (`/Game/Cat/UI/Title/WBP_Title.OnPressStart` _aswbp_title))))

(event `OpenMainMap`
  (`GameplayStatics.OpenLevel` (`self.MainMapName`)))

(event `PressGhostMode`
  (params (RankIndex :type Integer))
  ;[1 1 1] ゴーストモードのときはゴーストデータをロードしてからFadeOut
  (bind _asbp_main_game_instance (cast `/Game/Cat/BP/BP_MainGameInstance` (`GameplayStatics.GetGameInstance`)))
  (`MainGameInstance.LoadGameDataFromIndex` _asbp_main_game_instance RankIndex)
  (bind _wbp_fadeoutin (`self.GetWBP_FadeInOut`))
  (`/Game/Cat/UI/WBP_FadeOutIn.PlayFadeOut` _wbp_fadeoutin))

(event `self.LoadGhostTimeAndDoesGhostDataExists`
  (params (GhostTimes :type "Array of Float (single-precision) (by ref)") (DoesExists :type "Array of Boolean (by ref)"))
  (bind _wbp_ghostselect (`self.GetWBP_GhostSelect`))
  (`/Game/Cat/UI/Title/WBP_GhostSelect.InitGhostSelect` _wbp_ghostselect GhostTimes DoesExists))

(fn `GetTitlePlayer`
  (returns (`AsBP Title Pawn` :type "/Game/Cat/BP/Title/BP_TitlePawn Object Reference"))
  (bind _asbp_title_pawn (cast `/Game/Cat/BP/Title/BP_TitlePawn` (`GameplayStatics.GetPlayerPawn` 0)))
  (return _asbp_title_pawn))

(fn `GetWBP_FadeInOut`
  (returns (WBP_FadeOutIn :type "/Game/Cat/UI/WBP_FadeOutIn Object Reference"))
  (bind _aswbp_title (`self.GetWBP_Title`))
  (return (`/Game/Cat/UI/Title/WBP_Title.WBP_FadeOutIn` _aswbp_title)))

(fn `GetWBP_GhostSelect`
  (returns (WBP_GhostSelect :type "/Game/Cat/UI/Title/WBP_GhostSelect Object Reference"))
  (bind _aswbp_title (`self.GetWBP_Title`))
  (return (`/Game/Cat/UI/Title/WBP_Title.WBP_GhostSelect` _aswbp_title)))

(fn `GetWBP_Title`
  (returns (`AsWBP Title` :type "/Game/Cat/UI/Title/WBP_Title Object Reference"))
  (bind _aswbp_title (cast `/Game/Cat/UI/Title/WBP_Title` (`self.GetTitleWidget`)))
  (return _aswbp_title))

(fn `UserConstructionScript`)