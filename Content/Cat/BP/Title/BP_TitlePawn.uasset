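; Title-screen pawn that travels along a spline and signals when the player presses start.
; Each tick it accumulates distance from Speed and delta time, asks SplineActor for the location at that distance, and moves there without sweep, provided SplineActor is valid.
; Any key press calls OnPressStart; rotation is left untouched.
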(event `Key|AnyKey`
  (params (Key :type "Key Structure"))
  (:`Pressed`
    (`self.OnPressStart`)))

(event `self.ReceiveTick`
  (params (DeltaSeconds :type "Float (single-precision)"))
  (`/Engine/EditorBlueprintResources/StandardMacros.IsValid` (`self.SplineActor`)
    (:`Is Valid`
      (bind _output_get (set `self.MoveDistance` (+ (`self.MoveDistance`) (* DeltaSeconds (`self.Speed`)))))
      (bind _location (`/Game/Cat/BP/Title/BP_TitleSpline.GetCurrentLocation` (`self.SplineActor`) _output_get))
      (`self.K2_SetActorLocation` _location))))

(fn `UserConstructionScript`)