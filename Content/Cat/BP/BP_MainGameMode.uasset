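; BP_MainGameMode is the game mode that runs the race opening, extending parent prepare and start events.
; BeginPlay creates the fade widget.
; In the Main and TestMap levels, RacePrepare shows the start widget, plays a timed countdown with sound, then starts BGM and calls RaceStart.
; Tick prints dash points for debugging, and an unconnected branch holds TestMap ghost-mode spawning that never runs.
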(event `self.ReceiveBeginPlay`
  (`parent.ReceiveBeginPlay`)
  (bind _returnvalue (`|CreateWidget` "/Game/Cat/UI/WBP_FadeOutIn.WBP_FadeOutIn_C"))
  (`UserWidget.AddToViewport` _returnvalue 0)
  (set `self.FadeInOutWidget` _returnvalue))

(event `self.RacePrepare`
  (`/Game/Cat/BP/ActorMacroLibrary.IsCurrentLevelName` "Main"
    (:`true`
      _)
    (:`false`
      (`/Game/Cat/BP/ActorMacroLibrary.IsCurrentLevelName` "TestMap"
        (:`true`
          _))))
  (`parent.RacePrepare`)
  (bind _returnvalue (`|CreateWidget` "/Game/Cat/UI/WBP_Start.WBP_Start_C"))
  (`UserWidget.AddToViewport` _returnvalue 0)
  (`KismetSystemLibrary.Delay` 1.0)
  (`/Game/Cat/UI/WBP_Start.PlayCountDownAnimation` _returnvalue)
  (`GameplayStatics.PlaySound2D` "/Game/Cat/Sound/CountDown-2.CountDown-2" 1.0 1.0 0.0 null null)
  (`KismetSystemLibrary.Delay` 3.25)
  (`GameplayStatics.PlaySound2D` "/Game/Cat/Sound/BGM/MainGameBGM.MainGameBGM" 1.0 1.0 0.0 null null)
  (`self.RaceStart`))

(event `self.RaceStart`
  (`parent.RaceStart`))

(event `self.ReceiveTick`
  (params (DeltaSeconds :type "Float (single-precision)"))
  (`KismetSystemLibrary.PrintString` (`KismetStringLibrary.Conv_IntToString` (`self.GetCurrentDashPoint`))))

(fn `UserConstructionScript`)