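; BP_Cat is the player cat Blueprint for a racing game with a dash-point mechanic.
; Its live graph relays dash-point gain and decrease events to dispatchers, and the Pause input alternates race paused and unpaused broadcasts through a FlipFlop.
; The remaining logic is disconnected: per-level widget creation, a velocity-driven post-process blur using a dynamic material, and unused speed-to-FOV math.
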(event `self.ReceiveBeginPlay`)

(event `self.OnAddDashPointEvent`
  (params (CurrentPoint :type Integer) (MaxPoint :type Integer) (IsNotDashing :type Boolean))
  (`self.OnAddDashPoint` CurrentPoint MaxPoint IsNotDashing))

(event `InputAction|Pause` :paused true
  (params (Key :type "Key Structure"))
  (:`Pressed`
    (`self.OnPaused`)))

(event `OnPaused`
  (`/Engine/EditorBlueprintResources/StandardMacros.FlipFlop`
    (:`A`
      (`self.OnRacePaused`))
    (:`B`
      (`self.OnRaceUnPaused`))))

(event `self.OnDecreaseDashingPointEvent`
  (`self.OnDecreaseDashingPoint`))

(fn `UserConstructionScript`)