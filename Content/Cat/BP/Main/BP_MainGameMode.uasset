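; Race game mode for the cat game that drives HUD, music and level transitions from countdown to results.
; Handles parent race events, playing countdown, timer and goal widgets inside WBP_Cat and starting BGM on race start.
; BP_Cat delegates update the dash meter and toggle pause, while pause-menu delegates continue, restart or return to title.
; Level loads wait on fade-out callbacks, with the results map following the post-goal save.
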(event `self.ReceiveBeginPlay`
  (`parent.ReceiveBeginPlay`)
  (`|ExecutionSequence`
    (:`then_0`
      (`AudioComponent.Stop` (`self.BGM`))
      (bind _wbp_fadeoutin (`self.GetWBP_FadeOutIn`))
      (`/Game/Cat/UI/WBP_FadeOutIn.PlayFadeIn` _wbp_fadeoutin)
      (add `/Game/Cat/UI/WBP_FadeOutIn.OnFadeOut` _wbp_fadeoutin (delegate `OpenResultMap`))
      ;[1 1 1] Time更新ごとに呼び出すので変数化
      (bind _wbp_cat (`self.GetWBP_Cat`))
      (set `self.WBP_Time` (`/Game/Cat/UI/Main/WBP_Cat.WBP_Time` _wbp_cat)))
    (:`then_1`
      (bind _bp_cat (`self.GetBP_Cat`))
      (add `/Game/Cat/BP/Main/BP_Cat.OnAddDashPoint` _bp_cat (delegate `AddPoint`))
      (add `/Game/Cat/BP/Main/BP_Cat.OnDecreaseDashingPoint` _bp_cat (delegate `DecreaseDashingPoint`)))
    (:`then_2`
      (bind _bp_cat_2 (`self.GetBP_Cat`))
      (add `/Game/Cat/BP/Main/BP_Cat.OnRacePaused` _bp_cat_2 (delegate `CallRacePaused`))
      (add `/Game/Cat/BP/Main/BP_Cat.OnRaceUnPaused` _bp_cat_2 (delegate `CallRaceUnPaused`))
      (bind _wbp_pause (`self.GetWBP_Pause`))
      (add `/Game/Cat/UI/Main/WBP_Pause.OnContinueGame` _wbp_pause (delegate `ContinueGame`))
      (add `/Game/Cat/UI/Main/WBP_Pause.OnBackToTitle` _wbp_pause (delegate `BackToTitle`))
      (add `/Game/Cat/UI/Main/WBP_Pause.OnRestartGame` _wbp_pause (delegate `RestartGame`)))))

(event `OpenResultMap`
  (`GameplayStatics.OpenLevel` (`self.ResultMapName`)))

(event `DecreaseDashingPoint`
  ;[1 1 1] ダッシュ中にダッシュメーターを減少させる
  (bind _wbp_cat (`self.GetWBP_Cat`))
  (`/Game/Cat/UI/Main/WBP_Cat.DecreaseDashMeter` _wbp_cat))

(event `AddPoint`
  (params (Point :type Integer) (MaxPoint :type Integer) (IsNotDashing :type Boolean))
  ;[1 1 1] ダッシュポイントが更新されたときアニメーションを再生
  (bind _wbp_cat (`self.GetWBP_Cat`))
  (`/Game/Cat/UI/Main/WBP_Cat.AddDashPointMaterial` _wbp_cat Point MaxPoint IsNotDashing))

(event `BackToTitle`
  (bind _wbp_fadeoutin (`self.GetWBP_FadeOutIn`))
  (add `/Game/Cat/UI/WBP_FadeOutIn.OnFadeOut` _wbp_fadeoutin (delegate `OpenTitleMap`))
  (`/Game/Cat/UI/WBP_FadeOutIn.PlayFadeOut` _wbp_fadeoutin))

(event `ContinueGame`
  (bind _bp_cat (`self.GetBP_Cat`))
  (`/Game/Cat/BP/Main/BP_Cat.OnPaused` _bp_cat))

(event `RestartGame`
  (`self.RestartRace`)
  (bind _wbp_fadeoutin (`self.GetWBP_FadeOutIn`))
  (add `/Game/Cat/UI/WBP_FadeOutIn.OnFadeOut` _wbp_fadeoutin (delegate `OpenCurrentMap`))
  (`/Game/Cat/UI/WBP_FadeOutIn.PlayFadeOut` _wbp_fadeoutin))

(event `OpenTitleMap`
  (`GameplayStatics.OpenLevel` (`self.TitleMapName`)))

(event `CallRacePaused`
  (bind _wbp_cat (`self.GetWBP_Cat`))
  (`/Game/Cat/UI/Main/WBP_Cat.PlayShowPauseMenu` _wbp_cat)
  (set `PlayerController.bShowMouseCursor` true (`GameplayStatics.GetPlayerController` 0))
  (`AudioComponent.SetPaused` (`self.BGM`) true)
  (`self.RacePaused`))

(event `CallRaceUnPaused`
  (bind _wbp_cat (`self.GetWBP_Cat`))
  (`/Game/Cat/UI/Main/WBP_Cat.PlayUnShowPauseMenu` _wbp_cat)
  (set `PlayerController.bShowMouseCursor` false (`GameplayStatics.GetPlayerController` 0))
  (`AudioComponent.SetPaused` (`self.BGM`) false)
  (`self.RaceUnPaused`))

(event `OpenCurrentMap`
  (bind _returnvalue (`GameplayStatics.GetCurrentLevelName` true))
  (`GameplayStatics.OpenLevel` (`KismetStringLibrary.Conv_StringToName` _returnvalue)))

(event `self.RacePrepare`
  (`parent.RacePrepare`)
  (bind _wbp_start (`self.GetWBP_Start`))
  (add `/Game/Cat/UI/Main/WBP_Start.OnRaceStartEvent` _wbp_start (delegate `OnRaceStart`))
  (`KismetSystemLibrary.Delay` 1.0)
  (`/Game/Cat/UI/Main/WBP_Start.PlayCountDownAnimation` _wbp_start)
  (`GameplayStatics.PlaySound2D` "/Game/Cat/Sound/CountDown-2.CountDown-2" 1.0 1.0 0.0 null null))

(event `OnRaceStart`
  (`AudioComponent.Play` (`self.BGM`) 0.0)
  (`self.RaceStart`))

(event `self.GoalEvent`
  ;[1 1 1] ゴールした瞬間のイベント
  (`self.GetBP_Cat`)
  (bind _wbp_goal (`self.GetWBP_Goal`))
  (`/Game/Cat/UI/Main/WBP_Goal.PlayGoalAnimation` _wbp_goal))

(event `self.OnSavedEvent`
  ;[1 1 1] ゴール後セーブが終わった時のイベント
  (bind _wbp_fadeoutin (`self.GetWBP_FadeOutIn`))
  (`/Game/Cat/UI/WBP_FadeOutIn.PlayFadeOut` _wbp_fadeoutin))

(event `self.UpdateTimeCount`
  (params (CurrentTime :type "Float (single-precision)"))
  (`/Game/Cat/UI/Main/WBP_Time.SetTimeText` (`self.WBP_Time`) CurrentTime))

(fn `GetBP_Cat`
  (returns (`BP Cat` :type "/Game/Cat/BP/Main/BP_Cat Object Reference"))
  (bind _asbp_cat (cast `/Game/Cat/BP/Main/BP_Cat` (`GameplayStatics.GetPlayerCharacter` 0)))
  (return _asbp_cat))

(fn `GetWBP_Cat`
  (returns (`WBP Cat` :type "/Game/Cat/UI/Main/WBP_Cat Object Reference"))
  (bind _aswbp_cat (cast `/Game/Cat/UI/Main/WBP_Cat` (`self.GetCatWidget`)))
  (return _aswbp_cat))

(fn `GetWBP_FadeOutIn`
  (returns (WBP_FadeOutIn :type "/Game/Cat/UI/WBP_FadeOutIn Object Reference"))
  (bind _wbp_cat (`self.GetWBP_Cat`))
  (return (`/Game/Cat/UI/Main/WBP_Cat.WBP_FadeOutIn` _wbp_cat)))

(fn `GetWBP_Goal`
  (returns (WBP_Goal :type "/Game/Cat/UI/Main/WBP_Goal Object Reference"))
  (bind _wbp_cat (`self.GetWBP_Cat`))
  (return (`/Game/Cat/UI/Main/WBP_Cat.WBP_Goal` _wbp_cat)))

(fn `GetWBP_Pause`
  (returns (WBP_Pause :type "/Game/Cat/UI/Main/WBP_Pause Object Reference"))
  (bind _wbp_cat (`self.GetWBP_Cat`))
  (return (`/Game/Cat/UI/Main/WBP_Cat.WBP_Pause` _wbp_cat)))

(fn `GetWBP_Start`
  (returns (WBP_Start :type "/Game/Cat/UI/Main/WBP_Start Object Reference"))
  (bind _wbp_cat (`self.GetWBP_Cat`))
  (return (`/Game/Cat/UI/Main/WBP_Cat.WBP_Start` _wbp_cat)))

(fn `UserConstructionScript`)