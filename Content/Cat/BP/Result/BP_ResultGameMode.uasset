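; Game mode for the result screen, which shows the player's time in a ranking and leads back to the title map.
; BeginPlay fades in the WBP_Ranking widget and wires its events to BP_ResultPlayer, toggling whether any-key input is accepted.
; An any-key press makes the widget show its buttons, and the Go to Title button opens the title level.
; OnInitialRanking passes rank index, current time and ranking times to the widget.
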(event `self.ReceiveBeginPlay`
  (`parent.ReceiveBeginPlay`)
  (`|ExecutionSequence`
    (:`then_0`
      (bind _aswbp_ranking (`self.GetWBP_Ranking`))
      (`/Game/Cat/UI/WBP_FadeOutIn.PlayFadeIn` (`/Game/Cat/UI/Result/WBP_Ranking.WBP_FadeOutIn` _aswbp_ranking)))
    (:`then_1`
      (bind _asbp_result_player (`self.GetResultPlayer`))
      (add `/Game/Cat/BP/Result/BP_ResultPlayer.OnShowBtn` _asbp_result_player (delegate `ShowBtns`)))
    (:`then_2`
      (bind _aswbp_ranking_2 (`self.GetWBP_Ranking`))
      (add `/Game/Cat/UI/Result/WBP_Ranking.OnEnableAnyKey` _aswbp_ranking_2 (delegate `EnableAnyKeyEvent`))
      (add `/Game/Cat/UI/Result/WBP_Ranking.OnDisableAnyKey` _aswbp_ranking_2 (delegate `DisableAnyKeyEvent`))
      (add `/Game/Cat/UI/Result/WBP_Ranking.OnGotoTitleClicked` _aswbp_ranking_2 (delegate `OpenTitleMap`)))))

(event `ShowBtns`
  ;[1 1 1] AnyKeyが押されたら
  (bind _aswbp_ranking (`self.GetWBP_Ranking`))
  (`/Game/Cat/UI/Result/WBP_Ranking.PressAnyKeyEvent` _aswbp_ranking))

(event `EnableAnyKeyEvent`
  ;[1 1 1] Result表示中はAnyKeyの判定ができるようにする
  (bind _asbp_result_player (`self.GetResultPlayer`))
  (set `/Game/Cat/BP/Result/BP_ResultPlayer.bCanAnyKeyEvent` true _asbp_result_player))

(event `DisableAnyKeyEvent`
  ;[1 1 1] ボタン表示中はAnyKey判定しないように
  (bind _asbp_result_player (`self.GetResultPlayer`))
  (set `/Game/Cat/BP/Result/BP_ResultPlayer.bCanAnyKeyEvent` false _asbp_result_player))

(event `OpenTitleMap`
  ;[1 1 1] 「タイトルへ」が押されたらタイトルへ移動
  (`GameplayStatics.OpenLevel` (`self.TitleMapName`)))

(event `self.OnInitialRanking`
  (params (RankIndex :type Integer) (CurrentTime :type "Float (single-precision)") (RankingTimes :type "Array of Float (single-precision) (by ref)"))
  ;[1 1 1] リザルト画面のランキングを更新
  (bind _aswbp_ranking (`self.GetWBP_Ranking`))
  (`/Game/Cat/UI/Result/WBP_Ranking.InitRanking` _aswbp_ranking RankIndex CurrentTime RankingTimes))

(fn `GetResultPlayer`
  (returns (`AsBP Result Player` :type "/Game/Cat/BP/Result/BP_ResultPlayer Object Reference"))
  (bind _asbp_result_player (cast `/Game/Cat/BP/Result/BP_ResultPlayer` (`GameplayStatics.GetPlayerCharacter` 0)))
  (return _asbp_result_player))

(fn `GetWBP_Ranking`
  (returns (`AsWBP Ranking` :type "/Game/Cat/UI/Result/WBP_Ranking Object Reference"))
  (bind _aswbp_ranking (cast `/Game/Cat/UI/Result/WBP_Ranking` (`self.GetResultWidget`)))
  (return _aswbp_ranking))

(fn `UserConstructionScript`)